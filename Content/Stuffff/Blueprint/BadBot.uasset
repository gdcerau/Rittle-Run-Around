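; BadBot is a flipbook enemy that patrols back and forth along a spline from BeginPlay.
; Two timelines move the box collision and a right or left flipbook by spline distance, one forward and one in reverse.
; Five-second Delays on each timeline's Update swap the visible flipbook and start the other timeline, forming a loop.
; The collision hit handler only fetches LevelDatabaseActor instances; setting OnHit is disconnected.
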(event `self.ReceiveBeginPlay`
  (bind _spline (`self.Spline`))
  (bind _spline_2 (`self.Spline`))
  (`SceneComponent.SetHiddenInGame` (`self.BadBodFlipbookLeft`) true false)
  (bind (_direction _animationalpha) (`Timeline|Timeline_0` :!label _label)
    (:`Update`
      (bind _returnvalue (* (`SplineComponent.GetSplineLength` _spline_2) _animationalpha))
      (`SceneComponent.K2_SetWorldTransform` (`self.BadBotFlipbookRight`) (`KismetMathLibrary.MakeTransform` (`SplineComponent.GetLocationAtDistanceAlongSpline` _spline_2 _returnvalue "World") (`SplineComponent.GetRotationAtDistanceAlongSpline` _spline_2 _returnvalue "World")) false false)
      (`SceneComponent.K2_SetWorldTransform` (`self.BoxCollision`) (`KismetMathLibrary.MakeTransform` (`SplineComponent.GetLocationAtDistanceAlongSpline` _spline_2 _returnvalue "World") (`SplineComponent.GetRotationAtDistanceAlongSpline` _spline_2 _returnvalue "World")) false false)
      (`KismetSystemLibrary.Delay` 5.0)
      (`SceneComponent.SetHiddenInGame` (`self.BadBotFlipbookRight`) true false)
      (`SceneComponent.SetHiddenInGame` (`self.BadBodFlipbookLeft`) false false)
      (bind (_direction_2 _animationalpha_2) (`Timeline|Timeline_1` :!via `ReverseFromEnd`)
        (:`Update`
          (bind _returnvalue_2 (* (`SplineComponent.GetSplineLength` _spline) _animationalpha_2))
          (`SceneComponent.K2_SetWorldTransform` (`self.BoxCollision`) (`KismetMathLibrary.MakeTransform` (`SplineComponent.GetLocationAtDistanceAlongSpline` _spline _returnvalue_2 "World") (`SplineComponent.GetRotationAtDistanceAlongSpline` _spline _returnvalue_2 "World")) false false)
          (`SceneComponent.K2_SetWorldTransform` (`self.BadBodFlipbookLeft`) (`KismetMathLibrary.MakeTransform` (`SplineComponent.GetLocationAtDistanceAlongSpline` _spline _returnvalue_2 "World") (`SplineComponent.GetRotationAtDistanceAlongSpline` _spline _returnvalue_2 "World")) false false)
          (`KismetSystemLibrary.Delay` 5.0)
          (`SceneComponent.SetHiddenInGame` (`self.BadBodFlipbookLeft`) true false)
          (`SceneComponent.SetHiddenInGame` (`self.BadBotFlipbookRight`) false false)
          (goto _label :!via `PlayFromStart`))))))

(event `self.BoxCollision.OnComponentHit`
  (params (HitComponent :type "PrimitiveComponent Object Reference") (OtherActor :type "Actor Object Reference") (OtherComp :type "PrimitiveComponent Object Reference") (NormalImpulse :type "Vector Structure") (Hit :type "HitResult Structure (by ref)"))
  (bind _outactors (`GameplayStatics.GetAllActorsOfClass` "/Game/Stuffff/Blueprint/LevelDatabaseActor.LevelDatabaseActor_C")))

(fn `UserConstructionScript`)